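; Powerup pickup that sets its skeletal mesh material to show which kind of powerup it is.
; While SetMaterial is true, Tick maps WhichPowerup ranges to movement, health, armor, weapon shot or ammo, with sub-values picking variants.
; These values are not assigned here, and the range thresholds suggest weighted rolls.
; Each branch assigns SetMaterial to itself, so the flag never clears here and the material reapplies every frame.
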(event EventTick
  (params (DeltaSeconds :type Float%20%28single-precision%29))
  (bind _whichpowerup (Variables|Default|GetWhichPowerup))
  (bind _whichpowerup_2 (Variables|Default|GetWhichPowerup))
  (bind _whichweaponshottype (Variables|Default|GetWhichWeaponShotType))
  (bind _whichpowerup_3 (Variables|Default|GetWhichPowerup))
  (if (Variables|Default|GetbSetMaterial)
    (if (<= (Variables|Default|GetWhichPowerup) 15)
      (if (<= (Variables|Default|GetWhichMovementPowerup) 50)
        (Rendering|Material|SetMaterial (Variables|Default|GetSkeletalMesh) 0 "/Game/Materials/SprintPickupMaterial.SprintPickupMaterial")
        (Variables|Default|SetbSetMaterial (Variables|Default|GetbSetMaterial))
        (else
          (Rendering|Material|SetMaterial (Variables|Default|GetSkeletalMesh) 0 "/Game/Materials/JumpPickupMaterial.JumpPickupMaterial")
          (Variables|Default|SetbSetMaterial (Variables|Default|GetbSetMaterial))))
      (elif (and (> _whichpowerup_2 15) (<= _whichpowerup_2 40))
        (if (<= (Variables|Default|GetWhichHealthPowerup) 70)
          (Rendering|Material|SetMaterial (Variables|Default|GetSkeletalMesh) 0 "/Game/Materials/RedMaterial.RedMaterial")
          (Variables|Default|SetbSetMaterial (Variables|Default|GetbSetMaterial))
          (else
            (Rendering|Material|SetMaterial (Variables|Default|GetSkeletalMesh) 0 "/Game/Materials/HOTPickupMaterial.HOTPickupMaterial")
            (Variables|Default|SetbSetMaterial (Variables|Default|GetbSetMaterial))))
        (elif (and (> _whichpowerup 40) (<= _whichpowerup 60))
          (if (<= (Variables|Default|GetWhichArmorPowerup) 60)
            (Rendering|Material|SetMaterial (Variables|Default|GetSkeletalMesh) 0 "/Game/Materials/CommonMaterial.CommonMaterial")
            (Variables|Default|SetbSetMaterial (Variables|Default|GetbSetMaterial))
            (else
              (Rendering|Material|SetMaterial (Variables|Default|GetSkeletalMesh) 0 "/Game/Materials/LegendaryMaterial.LegendaryMaterial")
              (Variables|Default|SetbSetMaterial (Variables|Default|GetbSetMaterial))))
          (elif (and (> _whichpowerup_3 60) (<= _whichpowerup_3 70))
            (if (<= (Variables|Default|GetWhichWeaponShotType) 45)
              (Rendering|Material|SetMaterial (Variables|Default|GetSkeletalMesh) 0 "/Game/Materials/TripleShotPickup.TripleShotPickup")
              (Variables|Default|SetbSetMaterial (Variables|Default|GetbSetMaterial))
              (elif (and (> _whichweaponshottype 45) (<= _whichweaponshottype 80))
                (Rendering|Material|SetMaterial (Variables|Default|GetSkeletalMesh) 0 "/Game/Materials/AutomaticPickupMaterial.AutomaticPickupMaterial")
                (Variables|Default|SetbSetMaterial (Variables|Default|GetbSetMaterial))
                (else
                  (Rendering|Material|SetMaterial (Variables|Default|GetSkeletalMesh) 0 "/Game/Materials/ExplosivePickup.ExplosivePickup")
                  (Variables|Default|SetbSetMaterial (Variables|Default|GetbSetMaterial)))))
            (else
              (Rendering|Material|SetMaterial (Variables|Default|GetSkeletalMesh) 0 "/Game/Materials/AmmoPickup.AmmoPickup")
              (Variables|Default|SetbSetMaterial (Variables|Default|GetbSetMaterial)))))))))

(fn ConstructionScript)